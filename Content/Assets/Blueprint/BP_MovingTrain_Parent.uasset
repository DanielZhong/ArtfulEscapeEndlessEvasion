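; BP_MovingTrain_Parent is a train Blueprint that moves when the player character enters its trigger.
; An overlap of BP_Character with the Moving component sets CanMove, then clears it after a five-second delay.
; While CanMove is set, Tick shifts the Box component along its local X axis by a fixed per-frame step, without sweep or delta-time scaling.
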(event OnComponentBeginOverlap(Moving)
  (params (OverlappedComponent :type Primitive%20Component%20Object%20Reference) (OtherActor :type Actor%20Object%20Reference) (OtherComp :type Primitive%20Component%20Object%20Reference) (OtherBodyIndex :type Integer) (bFromSweep :type Boolean) (SweepResult :type Hit%20Result%20Structure%20%28by%20ref%29))
  (Utilities|Casting|CastToBP_Character OtherActor)
  (Variables|Default|SetCanMove true)
  (Utilities|FlowControl|Delay 5.0)
  (Variables|Default|SetCanMove false))

(event EventBeginPlay
  (|CallParentFunction) ; This node is disabled and will not be called.\nDrag off pins to build functionality.
)

(event Collision|EventActorBeginOverlap
  (params (OtherActor :type Actor%20Object%20Reference))
  (|CallParentFunction OtherActor) ; This node is disabled and will not be called.\nDrag off pins to build functionality.
)

(event EventTick
  (params (DeltaSeconds :type Float%20%28single-precision%29))
  (|CallParentFunction DeltaSeconds)
  (if (Variables|Default|GetCanMove)
    (Transformation|AddLocalOffset (Variables|Default|GetBox) "5.000000,0.000000,0.000000" false false)))

(fn ConstructionScript
  (|CallParentFunction))