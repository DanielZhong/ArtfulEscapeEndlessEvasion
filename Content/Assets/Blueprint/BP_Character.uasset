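; Player character for an auto-running game with coin collection, lateral steering, jumping, timed crouching and mouse-driven decal painting.
; BeginPlay sets up cursor, music, Enhanced Input and the coin HUD, while Tick pushes the capsule forward by a fixed per-frame offset without sweep.
; Painting line-traces from the deprojected cursor to spawn temporary surface decals.
; AddCoins updates the HUD counter, and Lost disables movement and shows the end screen.
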(event Input|EnhancedActionEvents|EnhancedInputActionIA_Move
  (params (ActionValue :type Float%20%28double-precision%29) (ElapsedSeconds :type Float%20%28double-precision%29) (TriggeredSeconds :type Float%20%28double-precision%29) (InputAction :type Input%20Action%20Object%20Reference :default "/Game/Assets/Blueprint/Input/IA_Move.IA_Move"))
  (if (Variables|Default|GetCanMove)
    (Pawn|Input|AddMovementInput (Math|Vector|GetRightVector (Variables|Collision|GetCapsuleComponent)) ActionValue false)))

(event Input|EnhancedActionEvents|EnhancedInputActionIA_Jump
  (params (ActionValue :type Boolean) (ElapsedSeconds :type Float%20%28double-precision%29) (TriggeredSeconds :type Float%20%28double-precision%29) (InputAction :type Input%20Action%20Object%20Reference :default "/Game/Assets/Blueprint/Input/IA_Jump.IA_Jump"))
  (if (Variables|Default|GetCanMove)
    (Character|Jump)))

(event Input|EnhancedActionEvents|EnhancedInputActionIA_Paint
  (params (ActionValue :type Float%20%28double-precision%29) (ElapsedSeconds :type Float%20%28double-precision%29) (TriggeredSeconds :type Float%20%28double-precision%29) (InputAction :type Input%20Action%20Object%20Reference :default "/Game/Assets/Blueprint/Input/IA_Paint.IA_Paint"))
  (bind _returnvalue (Game|GetPlayerController 0))
  (bind (_worldlocation _worlddirection) (Game|Player|ConvertMouseLocationToWorldSpace _returnvalue))
  (:Triggered
    (if (== ActionValue 1.0)
      (bind (_outhit _returnvalue_2) (Collision|LineTraceByChannel _worldlocation (+ _worldlocation (* _worlddirection 1.5e+03)) "TraceTypeQuery1" true 0 "None"))
      (if _returnvalue_2
        (Rendering|Decal|SpawnDecalatLocation "/Game/Assets/Materials/Decal01.Decal01" "50.000000,50.000000,50.000000" (.Location (Collision|BreakHitResult _outhit)) (Math|Conversions|RotationFromXVector (.Normal (Collision|BreakHitResult _outhit))) 2e+01)
        (Development|PrintString (Utilities|String|ToString(Vector) (.Location (Collision|BreakHitResult _outhit))))))))

(event Input|EnhancedActionEvents|EnhancedInputActionIA_Crouch
  (params (ActionValue :type Boolean) (ElapsedSeconds :type Float%20%28double-precision%29) (TriggeredSeconds :type Float%20%28double-precision%29) (InputAction :type Input%20Action%20Object%20Reference :default "/Game/Assets/Blueprint/Input/IA_Crouch.IA_Crouch"))
  (if (Variables|Default|GetCanMove)
    (Character|Crouch)
    (Transformation|AddLocalOffset (Variables|Character|GetMesh) "0.000000,0.000000,-1.000000" false false)
    (Utilities|FlowControl|Delay 1.0)
    (Character|UnCrouch)
    (Transformation|AddLocalOffset (Variables|Character|GetMesh) "0.000000,0.000000,1.000000" false false)))

(event EventBeginPlay
  (bind _as玩家控制器 (Utilities|Casting|CastToPlayerController (Pawn|GetController)))
  (Variables|/Script/Engine.PlayerController|SetbShowMouseCursor _as玩家控制器 true)
  (Audio|PlaySound2D "/Game/Assets/Music/BP_BGMusic.BP_BGMusic" 1.0 1.0 0.0 0 0)
  (bind _as玩家控制器_2 (Utilities|Casting|CastToPlayerController (Pawn|GetController)))
  (Utilities|IsValid (PlayerController|LocalPlayerSubsystems|GetEnhancedInputLocalPlayerSubsystem _as玩家控制器_2)
    (:Is%20Valid
      (Input|AddMappingContext (PlayerController|LocalPlayerSubsystems|GetEnhancedInputLocalPlayerSubsystem _as玩家控制器_2) "/Game/Assets/Blueprint/Input/IMC_SS.IMC_SS" 0 "(bIgnoreAllPressedKeysUntilRelease=True,bForceImmediately=False,bNotifyUserSettings=False)")
      (bind _returnvalue (Game|ConstructObjectfromClass "/Game/Assets/Blueprint/WBP_Coin.WBP_Coin_C"))
      (bind _output_get (Variables|Default|SetWBPUI _returnvalue))
      (UserInterface|Viewport|AddtoViewport _output_get 0)
      (Default|SetCoinNumber (Variables|Default|GetWBPUI)))))

(event Collision|EventActorBeginOverlap
  (params (OtherActor :type Actor%20Object%20Reference)))

(event EventTick
  (params (DeltaSeconds :type Float%20%28single-precision%29))
  (if (Variables|Default|GetCanMove)
    (Transformation|AddLocalOffset (Variables|Collision|GetCapsuleComponent) "4.000000,0.000000,0.000000" false false)))

(fn ConstructionScript)

(fn Lost
  (Variables|Default|SetCanMove false)
  (bind _returnvalue (UserInterface|CreateWidget "/Game/Assets/Blueprint/WBP_EndScreen.WBP_EndScreen_C"))
  (Variables|Default|SetWBPEndGame _returnvalue)
  (UserInterface|Viewport|AddtoViewport (Variables|Default|GetWBPEndGame) 0))

(fn AddCoins
  (bind _output_get (Variables|Default|SetCoinsCount (+ 1 (Variables|Default|GetCoinsCount))))
  (Default|SetCoinNumber (Variables|Default|GetWBPUI) _output_get))