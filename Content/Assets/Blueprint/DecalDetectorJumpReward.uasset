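; A jump-boost reward actor with a spinning cube, unlocked when enough DecalDetect actors gather around it.
; Each Tick it runs a sphere overlap around itself filtered to DecalDetect and checks the count against a threshold.
; Past the threshold it destroys itself and raises BP_Character's JumpZVelocity.
; The timed reset sits behind a Delay after DestroyActor, so it likely never runs.
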(event EventBeginPlay)

(event Collision|EventActorBeginOverlap
  (params (OtherActor :type Actor%20Object%20Reference)))

(event EventTick
  (params (DeltaSeconds :type Float%20%28single-precision%29))
  (bind _returnvalue (Game|GetPlayerCharacter 0))
  (bind _charactermovement (Variables|/Script/Engine.Character|GetCharacterMovement _returnvalue))
  (Transformation|AddLocalRotation (Variables|Default|GetCube) "0.000000,0.000000,3.000000" false false)
  (bind _outactors (Collision|SphereOverlapActors (Transformation|GetActorLocation) 1.5e+02 (Utilities|Array|MakeArray "ObjectTypeQuery1") "/Game/Assets/Blueprint/DecalDetect.DecalDetect_C"))
  (if (> (Utilities|Array|Length _outactors) 25)
    (Actor|DestroyActor)
    (Utilities|Casting|CastToBP_Character _returnvalue)
    (Variables|/Script/Engine.CharacterMovementComponent|SetJumpZVelocity _charactermovement 1e+03)
    (Utilities|FlowControl|Delay 8.0)
    (Variables|/Script/Engine.CharacterMovementComponent|SetJumpZVelocity _charactermovement 5.7e+02)))

(fn ConstructionScript)