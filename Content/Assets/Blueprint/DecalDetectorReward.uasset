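; DecalDetectorReward is a spinning cube that rewards the player once enough DecalDetect actors accumulate around it.
; Each Tick it rotates the cube and runs a 150-unit sphere overlap for WorldStatic actors of that class.
; When more than 25 are found, it destroys itself and permanently adds to the BP_Character's RunSpeed and CoinsCount.
; Debug sphere and count-print nodes are left disconnected.
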(event EventBeginPlay)

(event Collision|EventActorBeginOverlap
  (params (OtherActor :type Actor%20Object%20Reference)))

(event EventTick
  (params (DeltaSeconds :type Float%20%28single-precision%29))
  (Transformation|AddLocalRotation (Variables|Default|GetCube) "0.000000,3.000000,0.000000" false false)
  (bind _outactors (Collision|SphereOverlapActors (Transformation|GetActorLocation) 1.5e+02 (Utilities|Array|MakeArray "ObjectTypeQuery1") "/Game/Assets/Blueprint/DecalDetect.DecalDetect_C"))
  (if (> (Utilities|Array|Length _outactors) 25)
    (Actor|DestroyActor)
    (bind _asbp_character (Utilities|Casting|CastToBP_Character (Game|GetPlayerCharacter 0)))
    (Variables|/Game/Assets/Blueprint/BP_Character.BP_Character_C|SetRunSpeed _asbp_character (+ (Variables|/Game/Assets/Blueprint/BP_Character.BP_Character_C|GetRunSpeed _asbp_character) 1.5e+02))
    (Variables|/Game/Assets/Blueprint/BP_Character.BP_Character_C|SetCoinsCount _asbp_character (+ (Variables|/Game/Assets/Blueprint/BP_Character.BP_Character_C|GetCoinsCount _asbp_character) 5))))

(fn ConstructionScript)